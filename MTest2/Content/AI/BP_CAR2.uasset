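; BP_CAR2 is a car Blueprint, filed under AI, that slides along the world Y axis with no steering or decision logic.
; Tick nudges it one unit toward +Y every frame using SetActorLocation without sweep.
; A one-second Delay ignores re-triggers while pending, so the swept one-unit step back fires only about once per second, leaving net +Y drift.
; An AddMovementInput back-and-forth chain is unconnected.
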(event `self.ReceiveTick`
  (params (DeltaSeconds :type "Float (single-precision)"))
  (`self.K2_SetActorLocation` (+ (`self.K2_GetActorLocation`) (+ (0.0 1.0 0.0) 0.0)))
  (`KismetSystemLibrary.Delay` 1.0)
  (`self.K2_SetActorLocation` (+ (`self.K2_GetActorLocation`) (+ (0.0 -1.0 0.0) 0.0)) true))

(fn `UserConstructionScript`)